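; BP_TabletHolder is a puzzle socket that receives a numbered tablet from the player and lights up when the correct one is placed.
; PlaceObject, if the holder is empty, stores the number, rotates the actor, shows the tablet, enables its trigger and removes the player's equipped item.
; A matching number turns on the spotlight.
; Pickup and BeginPlay share one reset that empties the holder, disables the trigger and darkens the light.
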(event EventBeginPlay
  (Rendering|SetVisibility (Variables|Default|GetTablet1) false true)
  (Collision|SetCollisionEnabled (Variables|Default|GetTrigger) "NoCollision")
  (Rendering|Components|Light|SetIntensity (Variables|Default|GetSpotLight) 0.0)
  (Variables|Default|SetHasTablet false))

(event EventPickup
  (Rendering|SetVisibility (Variables|Default|GetTablet1) false true)
  (Collision|SetCollisionEnabled (Variables|Default|GetTrigger) "NoCollision")
  (Rendering|Components|Light|SetIntensity (Variables|Default|GetSpotLight) 0.0)
  (Variables|Default|SetHasTablet false))

(event EventPlaceObject
  (params (Direction :type Rotator :default "0, 0, 0") (Player :type BP%20First%20Person%20Character%20Object%20Reference) (TabletNumber :type Integer))
  (if (not (Variables|Default|GetHasTablet))
    (Variables|Default|SetCurrentTabletNumber TabletNumber)
    (Transformation|SetActorRotation Direction)
    (Rendering|SetVisibility (Variables|Default|GetTablet1) true true)
    (Collision|SetCollisionEnabled (Variables|Default|GetTrigger) "QueryAndPhysics")
    (Variables|Default|SetHasTablet true)
    (Default|RemoveEquippedItem Player)
    (if (== (Variables|Default|GetCorrectTabletNumber) TabletNumber)
      (Rendering|Components|Light|SetIntensity (Variables|Default|GetSpotLight) 2e+04))))

(fn ConstructionScript)