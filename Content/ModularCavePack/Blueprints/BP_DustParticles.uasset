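; Placeable dust particle effect from the Modular Cave Pack, configured through actor variables with no active runtime logic.
; The construction script pushes density, color, particle size range and a Z-axis gravity value into the FXDustParticles component's parameters.
; It also sizes SpawnAreaBox from the bounds variable, then feeds that box's world bounds extent back as the particle spawn area.
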(event EventBeginPlay)

(event Collision|EventActorBeginOverlap
  (params (OtherActor :type Actor%20Object%20Reference)))

(event EventTick
  (params (DeltaSeconds :type Float%20%28single-precision%29)))

(fn ConstructionScript
  (bind _fx_dustparticles (Variables|Default|GetFX_DustParticles))
  (Effects|Components|ParticleSystem|SetFloatParameter _fx_dustparticles "ParticleDensity" (Variables|Default|GetDensity))
  (Effects|Components|ParticleSystem|SetColorParameter _fx_dustparticles "Color" (Variables|Default|GetColor))
  (Effects|Components|ParticleSystem|SetFloatParameter _fx_dustparticles "MinParticleSize" (Variables|Default|GetMin%20Particle%20Size))
  (Effects|Components|ParticleSystem|SetFloatParameter _fx_dustparticles "MaxParticleSize" (Variables|Default|GetMax%20Particle%20Size))
  (Effects|Components|ParticleSystem|SetVectorParameter _fx_dustparticles "Gravity" (Math|Vector|MakeVector 0.0 0.0 (Variables|Default|GetGravity)))
  (Components|Box|SetBoxExtent (Variables|Default|GetSpawnAreaBox) (Variables|Default|GetSpawnAreaBounds) true)
  (Effects|Components|ParticleSystem|SetVectorParameter _fx_dustparticles "SpawnArea" (.BoxExtent (Collision|GetComponentBounds (Variables|Default|GetSpawnAreaBox)))))