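; Configurable torch prop for the Modular Cave Pack, set up entirely in the Construction Script with no active runtime logic.
; Lit toggles the fire FX and point light and sets the burn tint on a dynamic MI_Torch material, unless overridden by BurnAmount.
; Exposed variables drive flame color, particle scale, density and height, plus light settings.
; A sphere component's radius supplies the flame's spawn area.
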(event EventBeginPlay)

(event Collision|EventActorBeginOverlap
  (params (OtherActor :type Actor%20Object%20Reference)))

(event EventTick
  (params (DeltaSeconds :type Float%20%28single-precision%29)))

(fn ConstructionScript
  (bind _pointlight (Variables|Default|GetPointLight))
  (bind _fx_fire (Variables|Default|GetFX_Fire))
  (bind _boverrideburnamount (Variables|Advanced|GetbOverrideBurnAmount))
  (bind _pointlight_2 (Variables|Default|GetPointLight))
  (bind _fx_fire_2 (Variables|Default|GetFX_Fire))
  (Utilities|FlowControl|Sequence
    (:then_0
      ;[1 1 1] Create Dynamic Material
      (Utilities|FlowControl|DoOnce false
        (:Completed
          (bind _returnvalue (Rendering|Material|CreateDynamicMaterialInstance (Variables|Default|GetSM_Torch) 0 "/Game/ModularCavePack/Materials/MI_Torch.MI_Torch" "None" :!class /Script/Engine.PrimitiveComponent))
          (LocalVariables|SetDynamicMaterial _returnvalue))))
    (:then_1
      ;[1 1 1] Set Lit State
      (if (Variables|Default|GetLit)
        (Rendering|SetVisibility _fx_fire true false)
        (Rendering|SetVisibility _pointlight_2 true false)
        (if _boverrideburnamount
          (Rendering|Material|SetVectorParameterValue (LocalVariables|GetDynamicMaterial) "Tint" (Utilities|TintSlider (Variables|Advanced|GetBurnAmount)) :!class /Script/Engine.MaterialInstanceDynamic :!label _label)
          (else
            (Rendering|Material|SetVectorParameterValue :self (LocalVariables|GetDynamicMaterial) :ParameterName "Tint" :!class /Script/Engine.MaterialInstanceDynamic)))
        (else
          (Rendering|SetVisibility _fx_fire false false)
          (Rendering|SetVisibility _pointlight_2 false false)
          (if _boverrideburnamount
            (goto _label)
            (else
              (Rendering|Material|SetVectorParameterValue (LocalVariables|GetDynamicMaterial) "Tint" "(R=1.000000,G=1.000000,B=1.000000,A=1.000000)" :!class /Script/Engine.MaterialInstanceDynamic))))))
    (:then_2
      (Utilities|FlowControl|Sequence
        (:then_0
          ;[1 1 1] FX Settings
          (Effects|Components|ParticleSystem|SetColorParameter _fx_fire_2 "Color" (Variables|Default|GetFlameColor))
          (Effects|Components|ParticleSystem|SetFloatParameter _fx_fire_2 "ParticleScale" (Variables|Advanced|GetParticleScale))
          (Components|Sphere|SetSphereRadius (Variables|Default|GetSpawnAreaSphere) (Variables|Advanced|GetFlameAreaScale) true)
          (Effects|Components|ParticleSystem|SetFloatParameter _fx_fire_2 "SpawnArea" (Variables|/Script/Engine.SphereComponent|GetSphereRadius (Variables|Default|GetSpawnAreaSphere)))
          (Effects|Components|ParticleSystem|SetFloatParameter _fx_fire_2 "ParticleDensity" (Variables|Advanced|GetParticleDensity))
          (Effects|Components|ParticleSystem|SetFloatParameter _fx_fire_2 "ParticleLifeDuration" (Variables|Default|GetFlameHeight)))
        (:then_1
          ;[1 1 1] Light Settings
          (Rendering|Components|Light|SetIntensity _pointlight (Variables|Default|GetLight%20Intensity))
          (Rendering|Components|Light|SetLightColor _pointlight (Variables|Default|GetLight%20Color) true)
          (Rendering|Lighting|SetAttenuationRadius _pointlight (Variables|Default|GetLight%20Radius))
          (Class|LightComponent|SetTemperature _pointlight (Variables|Advanced|GetLight%20Temperature))
          (Rendering|Components|Light|SetCastShadows _pointlight (Variables|Advanced|GetbCastShadows)))))))