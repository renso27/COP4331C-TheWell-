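; BP_DripEffect is a placeable dripping-droplet effect from the modular cave pack.
; Its construction script pushes drip rate, droplet size, lifetime and color variables into the FXDrip particle component's parameters.
; It also sizes SpawnAreaBox from the SpawnArea variable and feeds that box's bounds extent to the effect as its spawn area.
; The event graph is empty, so the Blueprint adds no runtime logic.
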(event EventBeginPlay)

(event Collision|EventActorBeginOverlap
  (params (OtherActor :type Actor%20Object%20Reference)))

(event EventTick
  (params (DeltaSeconds :type Float%20%28single-precision%29)))

(fn ConstructionScript
  (bind _fx_drip (Variables|Default|GetFX_Drip))
  (bind _spawnareabox (Variables|Default|GetSpawnAreaBox))
  (bind _fx_drip_2 (Variables|Default|GetFX_Drip))
  (Effects|Components|ParticleSystem|SetFloatParameter _fx_drip "DripRate" (Variables|Default|GetDripRate))
  (Effects|Components|ParticleSystem|SetFloatParameter _fx_drip "DropletSize" (Variables|Default|GetDropletScale))
  (Effects|Components|ParticleSystem|SetColorParameter _fx_drip "Color" (Variables|Default|GetColor))
  (Components|Box|SetBoxExtent _spawnareabox (Variables|Default|GetSpawnArea) true)
  (Effects|Components|ParticleSystem|SetVectorParameter _fx_drip_2 "SpawnArea" (.BoxExtent (Collision|GetComponentBounds _spawnareabox)))
  (Effects|Components|ParticleSystem|SetFloatParameter _fx_drip_2 "DropletLife" (Variables|Default|GetDropletLife)))