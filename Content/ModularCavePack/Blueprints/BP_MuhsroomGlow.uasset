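; Glowing mushroom prop for the modular cave pack, pairing a point light with a dust particle effect.
; The construction script applies exposed intensity, color and radius to the light, then pushes density, color, size range and gravity into the particle system's parameters.
; A box component is resized from the spawn bounds, and its extent feeds the particles' spawn area.
; The event graph holds no active logic.
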(event EventBeginPlay)

(event Collision|EventActorBeginOverlap
  (params (OtherActor :type Actor%20Object%20Reference)))

(event EventTick
  (params (DeltaSeconds :type Float%20%28single-precision%29)))

(fn ConstructionScript
  (bind _pointlight (Variables|Default|GetPointLight))
  (bind _fx_dustparticles (Variables|Default|GetFX_DustParticles))
  (bind _spawnareabox (Variables|Default|GetSpawnAreaBox))
  (bind _boxextent (Collision|GetComponentBounds _spawnareabox))
  (Utilities|FlowControl|Sequence
    (:then_0
      ;[1 1 1] Light
      (Rendering|Components|Light|SetIntensity _pointlight (Variables|Light|GetLightIntensity))
      (Rendering|Components|Light|SetLightColor _pointlight (Variables|Light|GetLightColor) true)
      (Rendering|Lighting|SetAttenuationRadius _pointlight (Variables|Light|GetLightRadius)))
    (:then_1
      ;[1 1 1] VFX
      (Effects|Components|ParticleSystem|SetFloatParameter _fx_dustparticles "ParticleDensity" (Variables|VFX|GetDensity))
      (Effects|Components|ParticleSystem|SetColorParameter _fx_dustparticles "Color" (Variables|VFX|GetColor))
      (Effects|Components|ParticleSystem|SetFloatParameter _fx_dustparticles "MinParticleSize" (Variables|VFX|GetMin%20Particle%20Size))
      (Effects|Components|ParticleSystem|SetFloatParameter _fx_dustparticles "MaxParticleSize" (Variables|VFX|GetMax%20Particle%20Size))
      (Effects|Components|ParticleSystem|SetVectorParameter _fx_dustparticles "Gravity" (Math|Vector|MakeVector 0.0 0.0 (Variables|VFX|GetGravity)))
      (Components|Box|SetBoxExtent (Variables|Default|GetSpawnAreaBox) (Variables|VFX|GetSpawnAreaBounds) true)
      (Effects|Components|ParticleSystem|SetVectorParameter _fx_dustparticles "SpawnArea" (Math|Vector|MakeVector (.x _boxextent) (.y _boxextent) (.z _boxextent))))))